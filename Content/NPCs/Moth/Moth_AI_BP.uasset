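; Moth NPC AI controller that starts a player-chase behavior tree when AI perception reports an update for the player character.
; A perception update for a PrometheusCharacter writes its mesh location, raised by the capsule half-height, to the ChasePlayerData blackboard and sets CanSensePlayer true.
; It then runs ChasePlayerBehaviorTree, while other actors only log a message.
; Stimulus state is never checked, so losing sight also sets CanSensePlayer true.
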(event OnTargetPerceptionUpdated(AIPerception)
  (params (Actor :type Actor%20Object%20Reference) (Stimulus :type AI%20Stimulus%20Structure))
  (bind _asprometheus_character (Utilities|Casting|CastToPrometheusCharacter Actor)
    (:then
      (bind _blackboardcomponent (Class|AIController|UseBlackboard "/Game/NPCs/Behavior/ChasePlayerData.ChasePlayerData"))
      (AI|Components|Blackboard|SetValueasVector _blackboardcomponent (Utilities|String|StringToName (Variables|Default|GetPlayerLocation)) (+ (Math|Vector|MakeVector 0.0 0.0 (Components|Capsule|GetUnscaledCapsuleHalfHeight (Variables|/Script/Engine.Character|GetCapsuleComponent _asprometheus_character))) (Transformation|GetWorldLocation (Variables|/Script/Engine.Character|GetMesh _asprometheus_character))))
      (AI|Components|Blackboard|SetValueasBool _blackboardcomponent (Utilities|String|StringToName (Variables|Default|GetCanSensePlayer)) true)
      (Development|PrintString "Deteced Player or Lost Player")
      (AI|RunBehaviorTree "/Game/NPCs/Behavior/ChasePlayerBehaviorTree.ChasePlayerBehaviorTree"))
    (:CastFailed
      (Development|PrintString "Detected non-player, ignoring"))))

(fn ConstructionScript)