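; AI controller for the crow NPC that pursues the player while keeping a distance that grows with the player's light percent.
; Tick checks whether the first perceived actor is the player, updates the ChasePlayerData blackboard and calls RunBehaviorTree on every such tick.
; SetDesiredMoveLocation offsets the player's position toward the crow by light-scaled distance, and that point is written to the PlayerLocation key.
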(event EventTick
  (params (DeltaSeconds :type Float%20%28single-precision%29))
  (bind _returnvalue (Class|AIController|GetAIPerceptionComponent))
  (bind _outactors (Class|AIPerceptionComponent|GetCurrentlyPerceivedActors _returnvalue))
  (if (>= (Utilities|Array|Length _outactors) 1)
    (Utilities|Casting|CastToPrometheusCharacter (Utilities|Array|Get(acopy) _outactors)
      (:then
        (Variables|Default|SetHasSensedPlayer true)
        (CallFunction|SetDesiredMoveLocation)
        (AI|Components|Blackboard|SetValueasVector (stale EventBeginPlay _blackboardcomponent) (Utilities|String|StringToName (Variables|Default|GetPlayerLocation)) (Variables|Default|GetDesiredMoveLocation))
        (AI|Components|Blackboard|SetValueasBool (stale EventBeginPlay _blackboardcomponent) (Utilities|String|StringToName (Variables|Default|GetCanSensePlayer)) (Variables|Default|GetHasSensedPlayer))
        (AI|RunBehaviorTree "/Game/NPCs/Behavior/ChasePlayerBehaviorTree.ChasePlayerBehaviorTree"))
      (:CastFailed
        (Development|PrintString "Detected non-player, ignoring")))
    (else
      (Variables|Default|SetHasSensedPlayer false)
      (AI|Components|Blackboard|SetValueasBool (stale EventBeginPlay _blackboardcomponent) (Utilities|String|StringToName (Variables|Default|GetCanSensePlayer)) (Variables|Default|GetHasSensedPlayer)))))

(event EventBeginPlay
  (bind _blackboardcomponent (Class|AIController|UseBlackboard "/Game/NPCs/Behavior/ChasePlayerData.ChasePlayerData")))

(fn ConstructionScript)

(fn MovetoDesiredLocation
  (AI|Navigation|MovetoLocation (Variables|Default|GetDesiredMoveLocation) 1.0 true true false))

(fn SetDesiredMoveLocation
  (bind _asprometheus_character (Utilities|Casting|CastToPrometheusCharacter (Game|Player|GetPlayerPawn 0))
    (:then
      (bind _returnvalue (Class|PrometheusCharacter|GetLightPercent _asprometheus_character))
      (Development|PrintString (Utilities|String|Append "Player Location: " (Utilities|String|ToString(Vector) (+ (Math|Vector|MakeVector 0.0 0.0 (Components|Capsule|GetUnscaledCapsuleHalfHeight (Variables|/Script/Engine.Character|GetCapsuleComponent _asprometheus_character))) (Transformation|GetWorldLocation (Variables|/Script/Engine.Character|GetMesh _asprometheus_character))))) false false)
      (Development|PrintString (Utilities|String|Append "Desired Distance: " (Utilities|String|ToString(Float) (* _returnvalue (Variables|Default|GetDistanceAwayAtMaxLight)))) false false)
      (Development|PrintString (Utilities|String|Append "Desired Vector: " (Utilities|String|ToString(Vector) (* (Math|Vector|GetUnitDirection(Vector) (+ (Math|Vector|MakeVector 0.0 0.0 (Components|Capsule|GetUnscaledCapsuleHalfHeight (Variables|/Script/Engine.Character|GetCapsuleComponent _asprometheus_character))) (Transformation|GetWorldLocation (Variables|/Script/Engine.Character|GetMesh _asprometheus_character))) (Transformation|GetActorLocation (Pawn|GetControlledPawn))) (* _returnvalue (Variables|Default|GetDistanceAwayAtMaxLight))))) false false)
      (Development|PrintString (Utilities|String|Append "Desired Location: " (Utilities|String|ToString(Vector) (+ (* (Math|Vector|GetUnitDirection(Vector) (+ (Math|Vector|MakeVector 0.0 0.0 (Components|Capsule|GetUnscaledCapsuleHalfHeight (Variables|/Script/Engine.Character|GetCapsuleComponent _asprometheus_character))) (Transformation|GetWorldLocation (Variables|/Script/Engine.Character|GetMesh _asprometheus_character))) (Transformation|GetActorLocation (Pawn|GetControlledPawn))) (* _returnvalue (Variables|Default|GetDistanceAwayAtMaxLight))) (Transformation|GetWorldLocation (Variables|/Script/Engine.Character|GetMesh _asprometheus_character))))) false false)
      (Variables|Default|SetDesiredMoveLocation (+ (* (Math|Vector|GetUnitDirection(Vector) (+ (Math|Vector|MakeVector 0.0 0.0 (Components|Capsule|GetUnscaledCapsuleHalfHeight (Variables|/Script/Engine.Character|GetCapsuleComponent _asprometheus_character))) (Transformation|GetWorldLocation (Variables|/Script/Engine.Character|GetMesh _asprometheus_character))) (Transformation|GetActorLocation (Pawn|GetControlledPawn))) (* _returnvalue (Variables|Default|GetDistanceAwayAtMaxLight))) (Transformation|GetWorldLocation (Variables|/Script/Engine.Character|GetMesh _asprometheus_character)))))
    (:CastFailed
      (Development|PrintString "Detected non-player, ignoring"))))